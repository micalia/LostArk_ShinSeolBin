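; BP_OBJ_Table is a table object that can switch between a move state and a general state.
; On BeginPlay it creates a dynamic instance of the M_TableRound material and stores it in DynamMat.
; Mesh overlap begin and end events forward to BeginOverlapCallFunc and EndOverlapCallFunc, which are defined outside this file.
; Tick reapplies the mesh collision profile every frame, choosing AssignObj or GeneralModeAssignObj from the Move flag.
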(event OnComponentBeginOverlap(StaticMesh)
  (params (OverlappedComponent :type Primitive%20Component%20Object%20Reference) (OtherActor :type Actor%20Object%20Reference) (OtherComp :type Primitive%20Component%20Object%20Reference) (OtherBodyIndex :type Integer) (bFromSweep :type Boolean) (SweepResult :type Hit%20Result%20Structure%20%28by%20ref%29))
  (Class|AssignObj|BeginOverlapCallFunc))

(event OnComponentEndOverlap(StaticMesh)
  (params (OverlappedComponent :type Primitive%20Component%20Object%20Reference) (OtherActor :type Actor%20Object%20Reference) (OtherComp :type Primitive%20Component%20Object%20Reference) (OtherBodyIndex :type Integer))
  (Class|AssignObj|EndOverlapCallFunc))

(event EventTick
  (params (DeltaSeconds :type Float%20%28single-precision%29))
  (if (Variables|Default|GetbMove)
    (Collision|SetCollisionProfileName (Variables|Default|GetStaticMesh) "AssignObj" true :!class /Script/Engine.PrimitiveComponent)
    (else
      (Collision|SetCollisionProfileName (Variables|Default|GetStaticMesh) "GeneralModeAssignObj" true :!class /Script/Engine.PrimitiveComponent))))

(event EventBeginPlay
  (bind _returnvalue (Rendering|Material|CreateDynamicMaterialInstance (Variables|Default|GetStaticMesh) 0 "/Game/StarterContent/Props/Materials/M_TableRound.M_TableRound" "None" :!class /Script/Engine.PrimitiveComponent))
  (Variables|Default|SetdynamMat _returnvalue))

(fn ConstructionScript)