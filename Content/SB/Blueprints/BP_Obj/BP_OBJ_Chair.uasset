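; BP_OBJ_Chair is a chair object whose collision follows a Move flag, apparently for placing or moving it.
; On BeginPlay it stores a dynamic instance of M_Chair_1 in DynamMat.
; Mesh overlap begin and end events forward to BeginOverlapCallFunc and EndOverlapCallFunc, which are defined outside this file.
; Tick reapplies the collision profile every frame: AssignObj while Move is true, GeneralModeAssignObj otherwise.
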(event OnComponentBeginOverlap(StaticMeshComponent0)
  (params (OverlappedComponent :type Primitive%20Component%20Object%20Reference) (OtherActor :type Actor%20Object%20Reference) (OtherComp :type Primitive%20Component%20Object%20Reference) (OtherBodyIndex :type Integer) (bFromSweep :type Boolean) (SweepResult :type Hit%20Result%20Structure%20%28by%20ref%29))
  (Class|AssignObj|BeginOverlapCallFunc))

(event OnComponentEndOverlap(StaticMeshComponent0)
  (params (OverlappedComponent :type Primitive%20Component%20Object%20Reference) (OtherActor :type Actor%20Object%20Reference) (OtherComp :type Primitive%20Component%20Object%20Reference) (OtherBodyIndex :type Integer))
  (Class|AssignObj|EndOverlapCallFunc))

(event EventBeginPlay
  (bind _returnvalue (Rendering|Material|CreateDynamicMaterialInstance (Variables|Default|GetStaticMeshComponent0) 0 "/Game/SB/VictorianLivingRoom/Materials/M_Chair_1.M_Chair_1" "None" :!class /Script/Engine.PrimitiveComponent))
  (Variables|Default|SetdynamMat _returnvalue))

(event Collision|EventActorBeginOverlap
  (params (OtherActor :type Actor%20Object%20Reference)))

(event EventTick
  (params (DeltaSeconds :type Float%20%28single-precision%29))
  (if (Variables|Default|GetbMove)
    (Collision|SetCollisionProfileName (Variables|Default|GetStaticMeshComponent0) "AssignObj" true :!class /Script/Engine.PrimitiveComponent)
    (else
      (Collision|SetCollisionProfileName (Variables|Default|GetStaticMeshComponent0) "GeneralModeAssignObj" true :!class /Script/Engine.PrimitiveComponent))))

(fn ConstructionScript)