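; Bookcase object Blueprint that can be switched into a move state, with overlap detection through a box component.
; On BeginPlay it creates a dynamic cupboard material instance on its static mesh and stores it in DynamMat.
; Box overlap begin and end events forward to BeginOverlapCallFunc and EndOverlapCallFunc, which are defined outside these graphs.
; Every Tick it sets the mesh collision profile to AssignObj or GeneralModeAssignObj according to the Move flag.
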(event OnComponentBeginOverlap(Box)
  (params (OverlappedComponent :type Primitive%20Component%20Object%20Reference) (OtherActor :type Actor%20Object%20Reference) (OtherComp :type Primitive%20Component%20Object%20Reference) (OtherBodyIndex :type Integer) (bFromSweep :type Boolean) (SweepResult :type Hit%20Result%20Structure%20%28by%20ref%29))
  (Class|AssignObj|BeginOverlapCallFunc))

(event OnComponentEndOverlap(Box)
  (params (OverlappedComponent :type Primitive%20Component%20Object%20Reference) (OtherActor :type Actor%20Object%20Reference) (OtherComp :type Primitive%20Component%20Object%20Reference) (OtherBodyIndex :type Integer))
  (Class|AssignObj|EndOverlapCallFunc))

(event EventBeginPlay
  (bind _returnvalue (Rendering|Material|CreateDynamicMaterialInstance (Variables|Default|GetSM_cupboard3_StaticMeshComponent0) 0 "/Game/SB/VictorianLivingRoom/Materials/M_Cupboard.M_Cupboard" "None" :!class /Script/Engine.PrimitiveComponent))
  (Variables|Default|SetdynamMat _returnvalue))

(event EventTick
  (params (DeltaSeconds :type Float%20%28single-precision%29))
  (if (Variables|Default|GetbMove)
    (Collision|SetCollisionProfileName (Variables|Default|GetSM_cupboard3_StaticMeshComponent0) "AssignObj" true :!class /Script/Engine.PrimitiveComponent)
    (else
      (Collision|SetCollisionProfileName (Variables|Default|GetSM_cupboard3_StaticMeshComponent0) "GeneralModeAssignObj" true :!class /Script/Engine.PrimitiveComponent))))

(fn ConstructionScript)