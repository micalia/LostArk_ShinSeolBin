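; BP_OBJ_Window is a window object that appears to be movable, with a box trigger for detecting overlaps.
; On BeginPlay it creates a dynamic instance of M_Frame on the mesh's first material slot and stores it as DynamMat.
; Box begin and end overlaps are forwarded to BeginOverlapCallFunc and EndOverlapCallFunc, which are not defined here.
; Older overlap-counting and cannot-assign material logic remains in the graph but never runs.
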(event OnComponentBeginOverlap(Box)
  (params (OverlappedComponent :type Primitive%20Component%20Object%20Reference) (OtherActor :type Actor%20Object%20Reference) (OtherComp :type Primitive%20Component%20Object%20Reference) (OtherBodyIndex :type Integer) (bFromSweep :type Boolean) (SweepResult :type Hit%20Result%20Structure%20%28by%20ref%29))
  (Class|AssignObj|BeginOverlapCallFunc))

(event OnComponentEndOverlap(Box)
  (params (OverlappedComponent :type Primitive%20Component%20Object%20Reference) (OtherActor :type Actor%20Object%20Reference) (OtherComp :type Primitive%20Component%20Object%20Reference) (OtherBodyIndex :type Integer))
  (Class|AssignObj|EndOverlapCallFunc))

(event EventBeginPlay
  (bind _returnvalue (Rendering|Material|CreateDynamicMaterialInstance (Variables|Default|GetStaticMesh) 0 "/Game/StarterContent/Props/Materials/M_Frame.M_Frame" "None" :!class /Script/Engine.PrimitiveComponent))
  (Variables|Default|SetdynamMat _returnvalue))

(event EventTick
  (params (DeltaSeconds :type Float%20%28single-precision%29)))

(fn ConstructionScript)