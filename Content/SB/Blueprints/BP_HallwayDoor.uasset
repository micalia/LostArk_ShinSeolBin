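; Hallway door actor that sends the player to the CinemaInGame level when a Character overlaps its NextStageDoor component.
; The overlap sets flags on the FadeUI held by BP_CinemaInGameMode to fade to black, then opens the level after a short delay.
; A ChangeCollisionPreset event switches NextStageDoor to the OverlapAll profile, with no caller in this Blueprint.
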(event OnComponentBeginOverlap(NextStageDoor)
  (params (OverlappedComponent :type Primitive%20Component%20Object%20Reference) (OtherActor :type Actor%20Object%20Reference) (OtherComp :type Primitive%20Component%20Object%20Reference) (OtherBodyIndex :type Integer) (bFromSweep :type Boolean) (SweepResult :type Hit%20Result%20Structure%20%28by%20ref%29))
  (Utilities|Casting|CastToCharacter OtherActor)
  (bind _asbp_cinema_in_game_mode (Utilities|Casting|CastToBP_CinemaInGameMode (Game|GetGameMode)))
  (Variables|/Game/SB/UMG/WB_FadeInFadeOut.WB_FadeInFadeOut_C|SetfadeStart (Variables|/Game/SB/Blueprints/BP_CinemaInGameMode.BP_CinemaInGameMode_C|GetFadeUI _asbp_cinema_in_game_mode) true)
  (Variables|/Game/SB/UMG/WB_FadeInFadeOut.WB_FadeInFadeOut_C|SetfadeToBlackScreen (Variables|/Game/SB/Blueprints/BP_CinemaInGameMode.BP_CinemaInGameMode_C|GetFadeUI _asbp_cinema_in_game_mode) true)
  (Utilities|FlowControl|Delay 2.1)
  (Game|OpenLevel(byObjectReference) "/Game/SB/Levels/CinemaInGame.CinemaInGame"))

(event Custom|ChangeCollisionPreset
  (Collision|SetCollisionProfileName (Variables|Default|GetNextStageDoor) "OverlapAll" true :!class /Script/Engine.PrimitiveComponent))

(event EventBeginPlay)

(event Collision|EventActorBeginOverlap
  (params (OtherActor :type Actor%20Object%20Reference)))

(event EventTick
  (params (DeltaSeconds :type Float%20%28single-precision%29)))

(fn ConstructionScript)