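; In-game mode that ends the boss fight by moving to the EndCinemaInGame level once the boss dies.
; On BeginPlay it adds the fade widget to the viewport and caches the BP_Boss instance.
; While ChkHp is set, Tick polls boss HP; at zero it waits, hides top-level widgets, fades the camera and audio, then opens the level.
; ChkHp clears only after the latent delays and level-open call.
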(event EventBeginPlay
  (bind _returnvalue (UserInterface|CreateWidget "/Game/SB/UMG/WB_FadeInFadeOut.WB_FadeInFadeOut_C"))
  (bind _output_get (Variables|Default|SetFadeUI _returnvalue))
  (UserInterface|Viewport|AddtoViewport _output_get 3)
  (bind _returnvalue_2 (Actor|GetActorOfClass "/Game/TJ/Boss/BP_Boss.BP_Boss_C"))
  (Variables|Default|SetBossInstance _returnvalue_2))

(event EventTick
  (params (DeltaSeconds :type Float%20%28single-precision%29))
  (if (Variables|Default|GetbChkHp)
    (if (<= (Variables|/Game/TJ/Boss/BP_Boss.BP_Boss_C|GetHP (Variables|Default|GetBossInstance)) 0.0)
      (Utilities|FlowControl|Delay 4.0)
      (bind _foundwidgets (Widget|GetAllWidgetsOfClass "/Script/UMG.UserWidget" true))
      (for _array_element _foundwidgets
        (Widget|SetVisibility _array_element "Hidden"))
      (CameraFades|StartCameraFade :self (Game|GetPlayerCameraManager 0) :ToAlpha 1.0 :Duration 2.0 :bShouldFadeAudio true :bHoldWhenFinished true)
      (Utilities|FlowControl|Delay 3.0)
      (Game|OpenLevel(byObjectReference) "/Game/SB/Levels/EndCinemaInGame.EndCinemaInGame")
      (Variables|Default|SetbChkHp false))))

(fn ConstructionScript)