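; BP_CinemaBoss is the boss actor for a cinematic in which it smashes a door before the game moves to the in-game map.
; Separate events play the door-breaking montage and swap BP_Door for a spawned destroyed door with camera shake and sound.
; FadeCinema sets fade-to-black flags on the cinema game mode's FadeUI and opens the map after a delay, while ChangeLevelToInGame opens it immediately.
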(event Custom|DestroyDoorEvent
  (bind _returnvalue (Actor|GetActorOfClass "/Game/SB/Blueprints/BP_Door.BP_Door_C"))
  (Actor|DestroyActor _returnvalue)
  (Game|SpawnActorfromClass (Variables|Default|GetDestroyDoor) (Math|Transform|MakeTransform (Variables|Default|GetDestroyDoorPos) "0.000000,180.000000,0.000000" "1.000000,1.000000,1.000000") "Undefined" "MultiplyWithRoot" 0 0)
  (Class|PlayerCameraManager|StartCameraShakefromSource (Variables|/Script/Engine.PlayerController|GetPlayerCameraManager (Game|GetPlayerController 0)) "/Game/SB/Blueprints/DestroyDoorShake.DestroyDoorShake_C" 0 1.0 "CameraLocal" "0, 0, 0")
  (Audio|PlaySound2D "/Game/SB/Sounds/DestroyDoorSound.DestroyDoorSound" 1.0 1.0 0.0 0 0))

(event Custom|PlayDestroyEvent
  (Animation|Montage|PlayMontage (Variables|Default|GetSkeletalMesh) "/Game/SB/Blueprints/AM_Boss_DestroyDoor.AM_Boss_DestroyDoor" 1.0 0.0 ""))

(event Custom|ChangeLevelToInGame
  (Game|OpenLevel(byObjectReference) "/Game/SB/Levels/InGameMap.InGameMap"))

(event Custom|FadeCinema
  (bind _asbp_cinema_in_game_mode (Utilities|Casting|CastToBP_CinemaInGameMode (Game|GetGameMode)))
  (Variables|/Game/SB/UMG/WB_FadeInFadeOut.WB_FadeInFadeOut_C|SetfadeStart (Variables|/Game/SB/Blueprints/BP_CinemaInGameMode.BP_CinemaInGameMode_C|GetFadeUI _asbp_cinema_in_game_mode) true)
  (Variables|/Game/SB/UMG/WB_FadeInFadeOut.WB_FadeInFadeOut_C|SetfadeToBlackScreen (Variables|/Game/SB/Blueprints/BP_CinemaInGameMode.BP_CinemaInGameMode_C|GetFadeUI _asbp_cinema_in_game_mode) true)
  (Utilities|FlowControl|Delay 2.1)
  (Game|OpenLevel(byObjectReference) "/Game/SB/Levels/InGameMap.InGameMap"))

(fn ConstructionScript)