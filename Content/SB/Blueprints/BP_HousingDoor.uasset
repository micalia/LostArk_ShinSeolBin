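; BP_HousingDoor is a door trigger that sends the player to the BaseHousing level.
; When a Character overlaps NextStageDoor, it starts a fade to black through the housing game mode's FadeUI and saves assigned object data via LostArkGameInstance.
; After a short delay it opens the level.
; A ChangeCollisionPreset event switches the trigger to an overlap-all collision profile.
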(event OnComponentBeginOverlap(NextStageDoor)
  (params (OverlappedComponent :type Primitive%20Component%20Object%20Reference) (OtherActor :type Actor%20Object%20Reference) (OtherComp :type Primitive%20Component%20Object%20Reference) (OtherBodyIndex :type Integer) (bFromSweep :type Boolean) (SweepResult :type Hit%20Result%20Structure%20%28by%20ref%29))
  (Utilities|Casting|CastToCharacter OtherActor)
  (bind _asbp_housing_game_mode (Utilities|Casting|CastToBP_HousingGameMode (Game|GetGameMode)))
  (Variables|/Game/SB/UMG/WB_FadeInFadeOut.WB_FadeInFadeOut_C|SetfadeStart (Variables|/Game/SB/Blueprints/BP_HousingGameMode.BP_HousingGameMode_C|GetFadeUI _asbp_housing_game_mode) true)
  (Variables|/Game/SB/UMG/WB_FadeInFadeOut.WB_FadeInFadeOut_C|SetfadeToBlackScreen (Variables|/Game/SB/Blueprints/BP_HousingGameMode.BP_HousingGameMode_C|GetFadeUI _asbp_housing_game_mode) true)
  (bind _aslost_ark_game_instance (Utilities|Casting|CastToLostArkGameInstance (Game|GetGameInstance)))
  (Class|LostArkGameInstance|SaveAssignObjDatas _aslost_ark_game_instance)
  (Utilities|FlowControl|Delay 2.1)
  ;[1 1 1] 기존
  (Game|OpenLevel(byObjectReference) "/Game/SB/Levels/BaseHousing.BaseHousing"))

(event Custom|ChangeCollisionPreset
  (Collision|SetCollisionProfileName (Variables|Default|GetNextStageDoor) "OverlapAll" true :!class /Script/Engine.PrimitiveComponent))

(event EventBeginPlay)

(event Collision|EventActorBeginOverlap
  (params (OtherActor :type Actor%20Object%20Reference)))

(event EventTick
  (params (DeltaSeconds :type Float%20%28single-precision%29)))

(fn ConstructionScript)