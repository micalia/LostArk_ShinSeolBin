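; Manager for the ending housing cinematic, exposing events that trigger its staged visual and UI beats.
; BossOpacityStartFunc starts a timed Tick ramp that drives boss opacity and post-process black alpha together through two Material Parameter Collections.
; AppearLastWall spawns the final housing wall at a stored transform and reveals the BP_EndHousingNPC mesh.
; Separate events add the subtitle and ending credit widgets to the viewport.
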(event Custom|AppearLastWall
  (Game|SpawnActorfromClass (Variables|Default|GetEndHousingWallInstance) (Math|Transform|MakeTransform (Variables|Default|GetHousingLastWallPos) (Variables|Default|GetHousingLastWallRot) "1.000000,1.000000,1.000000") "Undefined" "MultiplyWithRoot" 0 0)
  (bind _returnvalue (Actor|GetActorOfClass "/Game/SB/Blueprints/EndCinema2/BP_EndHousingNPC.BP_EndHousingNPC_C"))
  (Rendering|SetVisibility (Variables|/Game/SB/Blueprints/EndCinema2/BP_EndHousingNPC.BP_EndHousingNPC_C|GetSkeletalMesh _returnvalue) true false))

(event Custom|WhatHappenSubtitle
  (bind _returnvalue (UserInterface|CreateWidget "/Game/SB/UMG/WB_Subtitle.WB_Subtitle_C"))
  (UserInterface|Viewport|AddtoViewport _returnvalue 0))

(event Custom|BossOpacityStartFunc
  (Variables|Default|SetbossOpacityStart true))

(event Custom|StartEndingCredit
  (bind _returnvalue (UserInterface|CreateWidget "/Game/SB/Blueprints/EndCinema2/WB_EndingCredit.WB_EndingCredit_C"))
  (UserInterface|Viewport|AddtoViewport _returnvalue 0))

(event EventTick
  (params (DeltaSeconds :type Float%20%28single-precision%29))
  (if (Variables|Default|GetbossOpacityStart)
    (bind _output_get (Variables|Default|SetOpacityCurrTime (+ DeltaSeconds (Variables|Default|GetOpacityCurrTime))))
    (if (> _output_get (Variables|Default|GetOpacityTime))
      (Variables|Default|SetbossOpacityStart false)
      (else
        (Rendering|Material|SetScalarParameterValue "/Game/SB/EndHousing/Materials/MPC_Opacity.MPC_Opacity" "BossOpacity" (/ _output_get (Variables|Default|GetOpacityTime)) :!class /Script/Engine.KismetMaterialLibrary)
        (Rendering|Material|SetScalarParameterValue "/Game/SB/Blueprints/EndCinema2/MPC_PostProessBlackOpacity.MPC_PostProessBlackOpacity" "BlackAlpha" (/ _output_get (Variables|Default|GetOpacityTime)) :!class /Script/Engine.KismetMaterialLibrary)))))

(fn ConstructionScript)