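; BP_EndCinemaPlayer is a player actor for the ending cinematic, with a staff and a magic-circle child actor.
; Tick pins the actor at a fixed height and continuously spins the circle.
; StaffUpDown moves the staff vertically by timeline, then shows the circle and lets Tick grow it flat up to a size limit.
; Nothing connected in this graph calls StaffUpDown; its delayed call is unwired.
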(event Custom|StaffUpDown
  (bind _output_get (Variables|Default|SetoriginStaffPos (Variables|/Script/Engine.SceneComponent|GetRelativeLocation (Variables|Default|GetStaff1))))
  (Variables|Default|SetDestStaffPos (Math|Vector|MakeVector (.x _output_get) (.y _output_get) -0.672825))
  (bind _newtrack_1 (Timeline|StaffPosTimeline Play)
    (:Update
      (Transformation|SetRelativeLocation (Variables|Default|GetStaff1) (Math|Vector|MakeVector (.X (Class|KismetMathLibrary|BreakVector3f (Variables|Default|GetoriginStaffPos))) (.Y (Class|KismetMathLibrary|BreakVector3f (Variables|Default|GetoriginStaffPos))) _newtrack_1) false false))
    (:Finished
      (Variables|Default|SetbStartSetScale true)
      (Rendering|SetVisibility (Variables|Default|GetChildActor) true false))))

(event EventTick
  (params (DeltaSeconds :type Float%20%28single-precision%29))
  (CallFunction|FixZaxisLocation)
  (CallFunction|RotateMagicCircle DeltaSeconds)
  (if (Variables|Default|GetbStartSetScale)
    (bind _output_get (Variables|Default|SetCurrScale (+ (Variables|Default|GetCurrScale) (* DeltaSeconds (Variables|Default|GetScaleSpeed)))))
    (if (< _output_get (Variables|Default|GetLimitScale))
      (Transformation|SetRelativeScale3D (Variables|Default|GetChildActor) (Math|Vector|MakeVector _output_get _output_get 0.0)))))

(event EventBeginPlay)

(fn ConstructionScript)

(fn FixZaxisLocation
  (bind _returnvalue (Transformation|GetActorLocation))
  (Transformation|SetActorLocation (Math|Vector|MakeVector (.x _returnvalue) (.y _returnvalue) 55.0) false false))

(fn RotateMagicCircle
  (params (A :type Float%20%28double-precision%29))
  (bind _output_get (Variables|Default|SetroateVal (+ (Variables|Default|GetroateVal) (* A (Variables|Default|GetroateSpeed)))))
  (Transformation|SetRelativeRotation (Variables|Default|GetChildActor) (Math|Rotator|MakeRotator 0.0 0.0 _output_get) false false))