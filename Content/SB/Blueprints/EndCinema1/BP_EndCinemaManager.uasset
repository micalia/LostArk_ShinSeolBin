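; BP_EndCinemaManager holds the scripted events for an end cinematic, including opening the BaseEndCinemaHousing level.
; Stone powder events find spawner actors to fire looping effects; EndStonePowder stops looping only on BP_SpawnFallingStonePowder.
; Staff events toggle BP_EndCinemaPlayer's two staff meshes, animation pause and staff up-down flag.
; A white-screen widget is created on BeginPlay, and once StartWhiteScreen fires, Tick ramps its opacity over OpacityTime.
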(event Custom|FallingStonePowder
  (bind _outactors (Actor|GetAllActorsOfClass "/Game/SB/Blueprints/EndCinema1/BP_SpawnFallingStonePowder.BP_SpawnFallingStonePowder_C"))
  (for _array_element _outactors
    (Default|ExecuteStonePowderEffect _array_element)
    (Variables|/Game/SB/Blueprints/EndCinema1/BP_SpawnFallingStonePowder.BP_SpawnFallingStonePowder_C|SetbIsLoop _array_element true)))

(event Custom|OpenLevelEndHousing
  (Game|OpenLevel(byObjectReference) "/Game/SB/Levels/BaseEndCinemaHousing.BaseEndCinemaHousing"))

(event Custom|StartWhiteScreen
  (Variables|Default|SetbWhiteScreenStart true))

(event Custom|ChangeStaffMesh
  (bind _returnvalue (Actor|GetActorOfClass "/Game/SB/Blueprints/EndCinema1/BP_EndCinemaPlayer.BP_EndCinemaPlayer_C"))
  (Variables|/Script/Engine.SkeletalMeshComponent|SetbPauseAnims (Variables|/Script/Engine.Character|GetMesh _returnvalue) true)
  (Variables|/Game/SB/Blueprints/EndCinema1/BP_EndCinemaPlayer.BP_EndCinemaPlayer_C|SetbStartStaffUpDown _returnvalue true)
  (Rendering|SetVisibility (Variables|/Game/SB/Blueprints/EndCinema1/BP_EndCinemaPlayer.BP_EndCinemaPlayer_C|GetStaff _returnvalue) false false)
  (Rendering|SetVisibility (Variables|/Game/SB/Blueprints/EndCinema1/BP_EndCinemaPlayer.BP_EndCinemaPlayer_C|GetStaff1 _returnvalue) true false))

(event Custom|OriginStaffMesh
  (bind _returnvalue (Actor|GetActorOfClass "/Game/SB/Blueprints/EndCinema1/BP_EndCinemaPlayer.BP_EndCinemaPlayer_C"))
  (Variables|/Script/Engine.SkeletalMeshComponent|SetbPauseAnims (Variables|/Script/Engine.Character|GetMesh _returnvalue) false)
  (Variables|/Game/SB/Blueprints/EndCinema1/BP_EndCinemaPlayer.BP_EndCinemaPlayer_C|SetbStartStaffUpDown _returnvalue false)
  (Rendering|SetVisibility (Variables|/Game/SB/Blueprints/EndCinema1/BP_EndCinemaPlayer.BP_EndCinemaPlayer_C|GetStaff _returnvalue) true false)
  (Rendering|SetVisibility (Variables|/Game/SB/Blueprints/EndCinema1/BP_EndCinemaPlayer.BP_EndCinemaPlayer_C|GetStaff1 _returnvalue) false false))

(event Custom|FallinStonePowder2
  (bind _outactors (Actor|GetAllActorsOfClass "/Game/SB/Blueprints/EndCinema1/BP_SpawnFallingStonePowder2.BP_SpawnFallingStonePowder2_C"))
  (for _array_element _outactors
    (Default|ExecuteStonePowderEffect _array_element)
    (Variables|/Game/SB/Blueprints/EndCinema1/BP_SpawnFallingStonePowder2.BP_SpawnFallingStonePowder2_C|SetbIsLoop _array_element true)))

(event Custom|EndStonePowder
  (bind _outactors (Actor|GetAllActorsOfClass "/Game/SB/Blueprints/EndCinema1/BP_SpawnFallingStonePowder.BP_SpawnFallingStonePowder_C"))
  (for _array_element _outactors
    (Variables|/Game/SB/Blueprints/EndCinema1/BP_SpawnFallingStonePowder.BP_SpawnFallingStonePowder_C|SetbIsLoop _array_element false)))

(event EventBeginPlay
  (bind _returnvalue (UserInterface|CreateWidget "/Game/SB/Blueprints/EndCinema1/WB_WhiteScreen.WB_WhiteScreen_C"))
  (bind _output_get (Variables|Default|SetWB_WhiteScreen _returnvalue))
  (UserInterface|Viewport|AddtoViewport _output_get 0))

(event EventTick
  (params (DeltaSeconds :type Float%20%28single-precision%29))
  (CallFunction|WhiteScreenAction DeltaSeconds))

(fn ConstructionScript)

(fn WhiteScreenAction
  (params (A :type Float%20%28double-precision%29))
  (if (Variables|Default|GetbWhiteScreenStart)
    (bind _output_get (Variables|Default|SetopacityCurrTime (+ A (Variables|Default|GetopacityCurrTime))))
    (Widget|SetRenderOpacity (Variables|Default|GetWB_WhiteScreen) (/ _output_get (Variables|Default|GetopacityTime)))))