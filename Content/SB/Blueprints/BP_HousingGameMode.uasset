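; Game mode for the housing level that spawns and possesses the player and gates the door behind an object-assignment quest.
; BeginPlay creates fade and dialogue widgets, shows the opening line, disables input and caches level actors.
; AssignQuestSuccess checks the AssignObj count, then outlines the door, changes its collision and triggers a Tick-driven, cubic-eased camera move to CamDest, ending in dialogue.
; RestoreCamPos resets the camera; save-game logic is unconnected.
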(event EventBeginPlay
  (bind _returnvalue (UserInterface|CreateWidget "/Game/SB/UMG/WB_FadeInFadeOut.WB_FadeInFadeOut_C"))
  (bind _output_get (Variables|Default|SetFadeUI _returnvalue))
  (UserInterface|Viewport|AddtoViewport _output_get 4)
  (bind _returnvalue_2 (UserInterface|CreateWidget "/Game/SB/UMG/WB_Dialogue.WB_Dialogue_C"))
  (bind _output_get_2 (Variables|Default|SetdialogueUI _returnvalue_2))
  (UserInterface|Viewport|AddtoViewport _output_get_2 3)
  (Variables|/Script/UMG.TextBlock|SetText (Variables|/Script/LostArk.Dialogue|GetTalkText (Variables|Default|GetdialogueUI)) (Utilities|Text|FormatText (Utilities|Text|ToText(String) (Utilities|Array|Get(acopy) (Variables|Default|Getdialogue))) (Utilities|Text|MakeLiteralText " 
")))
  (bind _returnvalue_3 (Actor|GetActorOfClass "/Game/SB/Blueprints/BP_HousingDoor.BP_HousingDoor_C"))
  (Variables|Default|SetHousingDoor _returnvalue_3)
  (bind _returnvalue_4 (Actor|GetActorOfClass "/Script/LostArk.CameraDest"))
  (Variables|Default|SetCamDest _returnvalue_4)
  (Input|DisableInput (Game|GetPlayerController 0) 0)
  (bind _returnvalue_5 (Actor|GetActorOfClass "/Game/SB/Blueprints/BP_HousingSpawnPoint.BP_HousingSpawnPoint_C"))
  (bind _returnvalue_6 (Game|SpawnActorfromClass "/Game/SB/Blueprints/BP_HousingPlayer.BP_HousingPlayer_C" (Transformation|GetActorTransform _returnvalue_5) "Undefined" "MultiplyWithRoot" 0 0))
  (Pawn|Possess (Game|GetPlayerController 0) _returnvalue_6)
  (Variables|Default|SetPlayerCam (Actor|GetComponentbyClass _returnvalue_6 "/Script/Engine.CameraComponent"))
  (Class|HousingGameMode|InitSpringArmLength)
  (Utilities|FlowControl|Delay 2.5)
  (Class|HousingGameMode|InitHousingDoor))

(event EventAssignQuestSuccess
  (bind _housingdoorinstance (Variables|Default|GetHousingDoorInstance))
  (bind _outactors (Actor|GetAllActorsOfClass "/Script/LostArk.AssignObj"))
  (if (>= (Utilities|Array|Length _outactors) (Variables|Default|GetAssignQuestCount))
    (if (not (Variables|Default|GetbQuestSuccess))
      (Rendering|SetVisibility (Variables|/Game/SB/Blueprints/BP_HousingDoor.BP_HousingDoor_C|GetOutlineArch _housingdoorinstance) true false)
      (Rendering|SetVisibility (Variables|/Game/SB/Blueprints/BP_HousingDoor.BP_HousingDoor_C|GetOutlineDoor _housingdoorinstance) true false)
      (Utilities|FlowControl|Delay 2.0)
      (Variables|Default|SetbQuestSuccess true)
      (Variables|Default|SetbFocusCameraMove true)
      (Input|DisableInput (Game|GetPlayerController 0) 0)
      (Variables|Default|SetPlayerCamOriginTransform (Transformation|GetWorldTransform (Variables|Default|GetPlayerCam)))
      (bind _returnvalue (Actor|GetActorOfClass "/Game/SB/Blueprints/BP_HousingDoor.BP_HousingDoor_C"))
      (Default|ChangeCollisionPreset _returnvalue))))

(event EventTick
  (params (DeltaSeconds :type Float%20%28single-precision%29))
  (bind _camdest (Variables|Default|GetCamDest))
  (bind _dialogueui (Variables|Default|GetdialogueUI))
  (bind _playercamorigintransform (Variables|Default|GetPlayerCamOriginTransform))
  (bind (_location _rotation) (Math|Transform|BreakTransform _playercamorigintransform))
  (if (Variables|Default|GetbFocusCameraMove)
    (Variables|Default|SetDoorFocusMoveCurrTime (+ DeltaSeconds (Variables|Default|GetDoorFocusMoveCurrTime)))
    (bind _returnvalue (Class|HousingGameMode|EaseinOutCubic (/ (Variables|Default|GetDoorFocusMoveCurrTime) (Variables|Default|GetDoorFocusMoveTime))))
    (if (< 1.0 (/ (Variables|Default|GetDoorFocusMoveCurrTime) (Variables|Default|GetDoorFocusMoveTime)))
      (Variables|Default|SetbFocusCameraMove false)
      (Variables|Default|SetDoorFocusMoveCurrTime 0.0)
      (Widget|SetVisibility _dialogueui "Visible")
      (Variables|/Script/UMG.TextBlock|SetText (Variables|/Script/LostArk.Dialogue|GetTalkText _dialogueui) (Utilities|Text|ToText(String) (Utilities|Array|Get(acopy) (Variables|Default|Getdialogue) 1)))
      (else
        (Transformation|SetWorldLocationAndRotation (Variables|Default|GetPlayerCam) (Math|Vector|Lerp(Vector) _location (Transformation|GetActorLocation _camdest) _returnvalue) (Math|Rotator|Lerp(Rotator) _rotation (Transformation|GetActorRotation _camdest) _returnvalue true) false false)))))

(event EventRestoreCamPos
  (Transformation|SetWorldTransform (Variables|Default|GetPlayerCam) (Variables|Default|GetPlayerCamOriginTransform) false false))

(event EventInitHousingDoor
  (bind _returnvalue (Actor|GetActorOfClass "/Game/SB/Blueprints/BP_HousingDoor.BP_HousingDoor_C"))
  (Variables|Default|SetHousingDoorInstance _returnvalue))

(fn ConstructionScript)