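; Game mode for the end cinema housing scene that opens the level with a fade from a white screen.
; On BeginPlay it adds a white screen widget to the viewport, calls LoadAssignObjDatas to load object data, and starts the fade.
; Tick accumulates elapsed time and linearly lowers the widget's render opacity until the fade duration is reached, then stops updating it without removing the widget.
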(event EventBeginPlay
  (bind _returnvalue (UserInterface|CreateWidget "/Game/SB/Blueprints/EndCinema2/WB_EndCineWhiteScreen.WB_EndCineWhiteScreen_C"))
  (bind _output_get (Variables|Default|SetWhiteScreen _returnvalue))
  (UserInterface|Viewport|AddtoViewport _output_get 3)
  (Class|EndCinemaGameMode|LoadAssignObjDatas)
  (Variables|Default|SetbFadeStart true))

(event EventTick
  (params (DeltaSeconds :type Float%20%28single-precision%29))
  (if (Variables|Default|GetbFadeStart)
    (bind _output_get (Variables|Default|SetopacityCurrTime (+ DeltaSeconds (Variables|Default|GetopacityCurrTime))))
    (if (< _output_get (Variables|Default|GetopacityTime))
      (Widget|SetRenderOpacity (Variables|Default|GetWhiteScreen) (- 1.0 (/ (Variables|Default|GetopacityCurrTime) (Variables|Default|GetopacityTime))))
      (else
        (Variables|Default|SetbFadeStart false)))))

(fn ConstructionScript)